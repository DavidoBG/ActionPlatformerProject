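; BP_ActionChar is a combat character with health, a faction, and stunned and defeated states.
; Its HitBox starts disabled, can be toggled by SetHitBoxCollision, and deals fixed damage to overlapped action characters of other factions.
; ReceiveAttack reduces health, then either jumps the anim instance to a stun node and starts a stun timer, or jumps to defeat and disables capsule collision.
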(event `self.ReceiveBeginPlay`
  (`self.SetHitBoxCollision` false)
  (set `self.CurrentHealth` (`self.MaxHealth`)))

(event `self.HitBox.OnComponentBeginOverlap`
  (params (OverlappedComponent :type "PrimitiveComponent Object Reference") (OtherActor :type "Actor Object Reference") (OtherComp :type "PrimitiveComponent Object Reference") (OtherBodyIndex :type Integer) (bFromSweep :type Boolean) (SweepResult :type "HitResult Structure (by ref)"))
  (bind _asbp_action_char (cast `/Game/Blueprints/Characters/BP_ActionChar` OtherActor))
  (if (!= (`/Game/Blueprints/Characters/BP_ActionChar.Faction` _asbp_action_char) (`self.Faction`))
    (`self.ReceiveAttack` _asbp_action_char 25.0)))

(fn `ClearStun`
  (set `self.IsStunned` false))

(fn `ReceiveAttack`
  (params (Damage :type "Float (double-precision)" :default 25.0))
  (if (not (`self.IsDefeated`))
    (set `self.CurrentHealth` (- (`self.CurrentHealth`) (`local.Damage`)))
    (if (<= (`self.CurrentHealth`) 0.0)
      (`PaperZDAnimInstance.JumpToNode` (`self.GetAnimInstance`) "JumpDefeated" "None")
      (set `self.IsDefeated` true)
      (`PrimitiveComponent.SetCollisionEnabled` (`self.CapsuleComponent`) "NoCollision")
      (else
        (set `self.IsStunned` true)
        (`PaperZDAnimInstance.JumpToNode` (`self.GetAnimInstance`) "JumpStunned" "None")
        (`KismetSystemLibrary.K2_SetTimerDelegate` (`|CreateDelegate` :!event `ClearStun`) (`self.StunLength`))))))

(fn `SetHitBoxCollision`
  (params (`Set Active` :type Boolean))
  (if `Set Active`
    (`PrimitiveComponent.SetCollisionEnabled` (`self.HitBox`) "QueryOnly")
    (else
      (`PrimitiveComponent.SetCollisionEnabled` (`self.HitBox`) "NoCollision"))))

(fn `UserConstructionScript`)